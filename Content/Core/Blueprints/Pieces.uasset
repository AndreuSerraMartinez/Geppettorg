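; Slime chunk actor tied to MainSlimeCharacter that damages the first Enemy3_mele or Enemy1 it overlaps, only once.
; Construction script randomly picks one of two meshes for the outer and inner slime components.
; After LifeTime, a timeline shrinks the actor's scale, then asks the player character to delete the chunk.
; In parallel, a short post-spawn delay sets CanRejoinAfterSpawn.
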(event EventBeginPlay
  ;[1 1 1] LifeSpan
  (Utilities|FlowControl|Sequence
    (:then_0
      (Utilities|FlowControl|Delay (Variables|Default|GetLifeTime))
      (bind _newtrack_0 (Timeline|Shrinck PlayFromStart)
        (:Update
          (Transformation|SetActorScale3D (Math|Conversions|ToVector(Float) _newtrack_0)))
        (:Finished
          (bind _asmain_slime_character (Utilities|Casting|CastToMainSlimeCharacter (Game|GetPlayerCharacter 0)))
          (Default|DeleteChunk _asmain_slime_character self))))
    (:then_1
      (Utilities|FlowControl|Delay 0.5)
      (Variables|Default|SetCanRejoinAfterSpawn true))))

(event Collision|EventActorBeginOverlap
  (params (OtherActor :type Actor%20Object%20Reference))
  (bind _asenemy_3_mele (Utilities|Casting|CastToEnemy3_mele OtherActor)
    (:then
      (if (not (Variables|Default|GetDamaged))
        (Default|DMG _asenemy_3_mele)
        (Variables|Default|SetDamaged true :!label _label)))
    (:CastFailed
      (bind _asenemy_1 (Utilities|Casting|CastToEnemy1 OtherActor))
      (if (not (Variables|Default|GetDamaged))
        (Default|DMG _asenemy_1)
        (goto _label)))))

(event EventTick
  (params (DeltaSeconds :type Float%20%28single-precision%29)))

(fn ConstructionScript
  (bind _slime (Variables|Default|GetSlime))
  (bind _slimeinside (Variables|Default|GetSlimeInside))
  (if (== (Math|Random|RandomInteger 2) 0)
    (Components|StaticMesh|SetStaticMesh _slime "/Game/Core/Models3D/Trossets1_low.Trossets1_low")
    (Components|StaticMesh|SetStaticMesh _slimeinside "/Game/Core/Models3D/Trossets1_low.Trossets1_low")
    (else
      (Components|StaticMesh|SetStaticMesh _slime "/Game/Core/Models3D/Trossets2_high.Trossets2_high")
      (Components|StaticMesh|SetStaticMesh _slimeinside "/Game/Core/Models3D/Trossets2_high.Trossets2_high"))))