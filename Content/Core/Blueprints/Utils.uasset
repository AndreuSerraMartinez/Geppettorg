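; Utility Blueprint that sorts an array of Checkpoint actors in place by their Data.Index using a recursive quicksort.
; QuickSortCheckpoint shuffles the array, then hands its full range to QuickSortCheckpointImpl.
; PartitionCheckpoint pivots on the last element and returns the split index for recursion.
; The second recursive call passes Low as its upper bound, so right-hand partitions stay unsorted.
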(fn QuickSortCheckpoint
  (params (Checkpoint :type Array%20of%20Actor%20Object%20References))
  (Utilities|Array|Shuffle Checkpoint)
  (CallFunction|QuickSortCheckpointImpl Checkpoint 0 (Utilities|Array|LastIndex Checkpoint)))

(fn QuickSortCheckpointImpl
  (params (Array :type Array%20of%20Actor%20Object%20References) (Low :type Integer) (High :type Integer))
  (if (not (or (>= Low High) (< High 0)))
    (bind _pivotindex (CallFunction|PartitionCheckpoint Array Low High))
    (CallFunction|QuickSortCheckpointImpl Array Low (- _pivotindex 1))
    (CallFunction|QuickSortCheckpointImpl Array (+ _pivotindex 1) Low)))

(fn PartitionCheckpoint
  (params (Array :type Array%20of%20Actor%20Object%20References) (Low :type Integer) (High :type Integer))
  (bind _ascheckpoint (Utilities|Casting|CastToCheckpoint (Utilities|Array|Get(acopy) Array High)))
  (LocalVariables|SetPivot (.index (Variables|/Game/Blueprints/Event/Checkpoints/Checkpoint.Checkpoint_C|GetData _ascheckpoint)))
  (LocalVariables|SetDiv (- Low 1))
  (for _index (range Low (- High 1))
    (bind _ascheckpoint_2 (Utilities|Casting|CastToCheckpoint (Utilities|Array|Get(acopy) Array _index)))
    (if (not (> (.index (Variables|/Game/Blueprints/Event/Checkpoints/Checkpoint.Checkpoint_C|GetData _ascheckpoint_2)) (LocalVariables|GetPivot)))
      (bind _result (Math|Integer|IncrementInt (LocalVariables|GetDiv))
        (:%20%20
          (Utilities|Array|Swap Array _result _index)))))
  (bind _result_2 (Math|Integer|IncrementInt (LocalVariables|GetDiv))
    (:%20%20
      (Utilities|Array|Swap Array _result_2 High)
      (return (LocalVariables|GetDiv)))))