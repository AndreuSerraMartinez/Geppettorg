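; Cactus enemy that turns toward and shoots at the nearest target in its range sphere, either the player's main slime or a slime piece.
; A self-repeating LookingAt loop eases its yaw, while Tick separately aims the spawn point and fires after an anticipation scale timeline, gated by cooldown.
; DMG updates the health bar and flashes the material; at zero HP it notifies its spawner if spawned, then shrinks away.
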(event Custom|LookingAt
  (bind _rangespherecollision (Variables|Default|GetRangeSphereCollision))
  (bind _overlappingactors (Collision|GetOverlappingActors _rangespherecollision "/Game/Core/Blueprints/Pieces.Pieces_C" :!class /Script/Engine.PrimitiveComponent))
  (Variables|Anim|SetInitRoot (Transformation|GetActorRotation))
  (if (Utilities|Array|IsValidIndex _overlappingactors)
    (for (_array_element _array_index) _overlappingactors
      (if (< (Transformation|GetDistanceTo _array_element self) (Variables|Default|GetClosestDistance))
        (Variables|Default|SetClosestSlime _array_index)
        (Variables|Default|SetClosestDistance (Transformation|GetDistanceTo _array_element self))))
    (if (< (Transformation|GetDistanceTo (Variables|Default|GetMain%20Slime) self) (Variables|Default|GetClosestDistance))
      (Variables|Anim|SetRotationToLookAt (Math|Conversions|RotationFromXVector (- (Transformation|GetActorLocation (Variables|Default|GetMain%20Slime)) (Transformation|GetWorldLocation (Variables|Default|GetSpawn_projectile)))) :!label _label)
      (bind _newtrack_0 (Timeline|LookAt PlayFromStart)
        (:Update
          (Transformation|SetActorRotation (Math|Rotator|MakeRotator (.roll (Transformation|GetActorRotation)) 0.0 (.yaw (Math|Rotator|Lerp(Rotator) (Variables|Anim|GetInitRoot) (Variables|Anim|GetRotationToLookAt) _newtrack_0)))))
        (:Finished
          (Variables|Default|SetClosestSlime 0 :!label _label_2)
          (Variables|Default|SetClosestDistance 1e+04)
          (Utilities|FlowControl|Delay 1.0)
          (CallFunction|Lookingat)))
      (else
        (Variables|Anim|SetRotationToLookAt (Math|Conversions|RotationFromXVector (- (Transformation|GetActorLocation (Utilities|Array|Get(acopy) _overlappingactors (Variables|Default|GetClosestSlime))) (Transformation|GetWorldLocation (Variables|Default|GetSpawn_projectile)))))
        (Timeline|LookAt PlayFromStart)))
    (elif (Utilities|Array|IsValidIndex (Collision|GetOverlappingActors (Variables|Default|GetRangeSphereCollision) "/Game/Core/Blueprints/MainSlimeCharacter.MainSlimeCharacter_C" :!class /Script/Engine.PrimitiveComponent))
      (goto _label)
      (else
        (goto _label_2)))))

(event Custom|DMG
  (bind _spawner (Variables|Default|GetSpawner))
  ;[1 0 0] DMG
  (Math|Integer|DecrementInt (Variables|Default|GetHP)
    (:%20%20
      (Rendering|Material|SetMaterial (Variables|Default|GetCactus) 0 "/Game/ArtPacks/NatureUnreal/Materials/Foliage/MI_Flower_05.MI_Flower_05")
      (Niagara|SpawnSystematLocation "/Game/VFX/SlashHit/FX_Hit.FX_Hit" (Transformation|GetActorLocation) "0, 0, 0" "1.000000,1.000000,1.000000" false)
      (Variables|/Game/Blueprints/Widgets/HealthBar.HealthBar_C|SetHealth (Variables|Default|GetHealthBar) (Math|Conversions|ToFloat(Integer) (Variables|Default|GetHP)))
      (if (<= (Variables|Default|GetHP) 0)
        ;;[1 0 0.04513] TODO - no cura no?
        (bind _asmain_slime_character (Utilities|Casting|CastToMainSlimeCharacter (Game|GetPlayerCharacter 0)))
        (Default|AddLife _asmain_slime_character 0.0)
        (if (Variables|Default|GetSpawned)
          (Utilities|FlowControl|DoOnce false
            (:Completed
              (Math|Integer|DecrementInt (Variables|/Game/Blueprints/SpawnerWaves.SpawnerWaves_C|GetEnemyAlive _spawner)
                (:%20%20
                  (Default|CheckEnemyLeft _spawner))))))
        (Game|SpawnActorfromClass "/Game/VFX/EnemyDie/BP_EnemyDie.BP_EnemyDie_C" (Transformation|GetActorTransform) "Undefined" 0 0)
        (Audio|PlaySoundatLocation "/Game/Sounds/SFX/AlphaPlaceHolder/temp_poofDie.temp_poofDie" (Transformation|GetActorLocation) "0, 0, 0" 1.0 1.0 0.0 0 0 0 0)
        (bind _newtrack_0 (Timeline|Timeline PlayFromStart)
          (:Update
            (Transformation|SetActorScale3D (Math|Conversions|ToVector(Float) _newtrack_0)))
          (:Finished
            (Actor|DestroyActor)))
        (else
          (Utilities|FlowControl|Delay 0.2)
          (Rendering|Material|SetMaterial (Variables|Default|GetCactus) 0 "/Game/Characters/Enemies/Cactus/Cactus_low.Cactus_low"))))))

(event EventBeginPlay
  (bind _returnvalue (Transformation|GetActorRotation))
  (bind _returnvalue_2 (Transformation|GetActorScale3D))
  (CallFunction|Lookingat)
  ;[1 1 1] HUD Health
  (bind _ashealth_bar (Utilities|Casting|CastToHealthBar (UserInterface|GetUserWidgetObject (Variables|Default|GetWidget)))
    (:then
      (bind _output_get (Variables|Default|SetHealthBar _ashealth_bar))
      (bind _output_get_2 (Variables|/Game/Blueprints/Widgets/HealthBar.HealthBar_C|SetMaxHealth _output_get (Math|Conversions|ToFloat(Integer) (Variables|Default|GetHP))))
      (Variables|/Game/Blueprints/Widgets/HealthBar.HealthBar_C|SetHealth _output_get _output_get_2))
    (:CastFailed
      _))
  (bind _asmain_slime_character (Utilities|Casting|CastToMainSlimeCharacter (Game|GetPlayerCharacter 0)))
  (Variables|Default|SetMain%20Slime _asmain_slime_character)
  ;[1 1 1] Animations
  (bind (_direction _rotation _height) (Timeline|Animation PlayFromStart)
    (:Update
      (Transformation|SetActorRotation (Math|Rotator|MakeRotator (* (Variables|Anim|GetDegreeRotationAnim) _rotation) (.pitch _returnvalue) (.yaw _returnvalue)))
      (Transformation|SetActorScale3D (Math|Vector|MakeVector (.x _returnvalue_2) (.y _returnvalue_2) _height)))))

(event EventTick
  (params (DeltaSeconds :type Float%20%28single-precision%29))
  (bind _rangespherecollision (Variables|Default|GetRangeSphereCollision))
  (bind _overlappingactors (Collision|GetOverlappingActors _rangespherecollision "/Game/Core/Blueprints/Pieces.Pieces_C" :!class /Script/Engine.PrimitiveComponent))
  (if (Variables|Default|GetCanShoot)
    (Variables|Default|SetClosestSlime 0)
    (Variables|Default|SetClosestDistance 1e+04)
    (if (Utilities|Array|IsValidIndex _overlappingactors)
      (for (_array_element _array_index) _overlappingactors
        (if (< (Transformation|GetDistanceTo _array_element self) (Variables|Default|GetClosestDistance))
          (Variables|Default|SetClosestSlime _array_index)
          (Variables|Default|SetClosestDistance (Transformation|GetDistanceTo _array_element self))))
      (if (< (Transformation|GetDistanceTo (Variables|Default|GetMain%20Slime) self) (Variables|Default|GetClosestDistance))
        (Transformation|SetWorldRotation (Variables|Default|GetSpawn_projectile) (Math|Rotator|MakeRotator 0.0 0.0 (.yaw (Math|Conversions|RotationFromXVector (- (Transformation|GetActorLocation (Variables|Default|GetMain%20Slime)) (Transformation|GetWorldLocation (Variables|Default|GetSpawn_projectile)))))) false false :!label _label)
        (else
          (Transformation|SetWorldRotation (Variables|Default|GetSpawn_projectile) (Math|Rotator|MakeRotator 0.0 0.0 (.yaw (Math|Conversions|RotationFromXVector (- (Transformation|GetActorLocation (Utilities|Array|Get(acopy) _overlappingactors (Variables|Default|GetClosestSlime))) (Transformation|GetWorldLocation (Variables|Default|GetSpawn_projectile)))))) false false)))
      (Utilities|FlowControl|Sequence
        (:then_0
          (Variables|Default|SetClosestSlime 0)
          (Variables|Default|SetClosestDistance 1e+04)
          (Variables|Default|SetCanShoot false)
          ;[1 1 1] cooldown
          (Utilities|FlowControl|Delay (Variables|Default|GetCooldown))
          (Variables|Default|SetCanShoot true))
        (:then_1
          (bind _size (Timeline|Anticipation PlayFromStart)
            (:Update
              (Transformation|SetActorScale3D (Math|Vector|MakeVector _size _size (.z (Transformation|GetActorScale3D)))))
            (:Finished
              (Game|SpawnActorfromClass "/Game/Characters/Enemies/Projectile1.Projectile1_C" (Transformation|GetWorldTransform (Variables|Default|GetSpawn_projectile)) "Undefined" 0 0)))))
      (elif (Utilities|Array|IsValidIndex (Collision|GetOverlappingActors (Variables|Default|GetRangeSphereCollision) "/Game/Core/Blueprints/MainSlimeCharacter.MainSlimeCharacter_C" :!class /Script/Engine.PrimitiveComponent))
        (goto _label)))))

(fn ConstructionScript)