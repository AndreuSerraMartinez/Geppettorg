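; Talkable slime NPC that turns to face the player every tick and shows a widget while the player is in its trigger zone.
; Each Talk call advances through the Dialogue array in a D_Base UI, created when none is valid with a portrait texture matched to the mesh material.
; Talking freezes player movement and flags IsInDialogue; running out of lines restores movement, removes the UI and hides the widget.
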(event OnComponentBeginOverlap(TriggerZone)
  (params (OverlappedComponent :type Primitive%20Component%20Object%20Reference) (OtherActor :type Actor%20Object%20Reference) (OtherComp :type Primitive%20Component%20Object%20Reference) (OtherBodyIndex :type Integer) (bFromSweep :type Boolean) (SweepResult :type Hit%20Result%20Structure%20%28by%20ref%29))
  (Utilities|Casting|CastToMainSlimeCharacter OtherActor)
  (Rendering|SetVisibility (Variables|Default|GetWidget) true false))

(event OnComponentEndOverlap(TriggerZone)
  (params (OverlappedComponent :type Primitive%20Component%20Object%20Reference) (OtherActor :type Actor%20Object%20Reference) (OtherComp :type Primitive%20Component%20Object%20Reference) (OtherBodyIndex :type Integer))
  (Utilities|Casting|CastToMainSlimeCharacter OtherActor)
  (Rendering|SetVisibility (Variables|Default|GetWidget) false false)
  (if (< (Utilities|Array|Length (Variables|Default|GetDialogue)) (Variables|Default|GetTalkIndex))
    (Variables|Default|SetTalkIndex -1)))

(event EventTick
  (params (DeltaSeconds :type Float%20%28single-precision%29))
  (bind _self self)
  ;[1 1 1] Mirar al player
  (Transformation|SetActorRotation _self (Math|Rotator|FindLookatRotation (Transformation|GetActorLocation _self) (Transformation|GetActorLocation (Game|GetPlayerCharacter 0)))))

(event EventTalk
  (bind _asmain_slime_character (Utilities|Casting|CastToMainSlimeCharacter (Game|GetPlayerCharacter 0)))
  (Variables|/Script/Engine.CharacterMovementComponent|SetMaxWalkSpeed (Variables|/Script/Engine.Character|GetCharacterMovement _asmain_slime_character) 0.0)
  (Variables|/Game/Core/Blueprints/MainSlimeCharacter.MainSlimeCharacter_C|SetIsInDialogue _asmain_slime_character true)
  (Math|Integer|IncrementInt (Variables|Default|GetTalkIndex)
    (:%20%20
      (if (< (Variables|Default|GetTalkIndex) (Utilities|Array|Length (Variables|Default|GetDialogue)))
        (Variables|Default|GetUI_Base
          (:then
            (Rendering|Components|TextRender|SetText (Variables|/Game/UI/Dialogues/D_Z0/D_Base.D_Base_C|Getdialogue (Variables|Default|GetUI_Base)) (Utilities|Text|ToText(String) (Utilities|Array|Get(acopy) (Variables|Default|GetDialogue) (Variables|Default|GetTalkIndex))) :!label _label))
          (:else
            (bind _returnvalue (UserInterface|CreateWidget "/Game/UI/Dialogues/D_Z0/D_Base.D_Base_C" (Game|GetPlayerController 0) (Variables|Default|GetNPC%20name) "" (Variables|Default|GetTextureSlime)))
            (bind _output_get (Variables|Default|SetUI_Base _returnvalue))
            (if (== (Rendering|Material|GetMaterial (Variables|Character|GetMesh) 0) "/Game/Characters/NPCs/M_Slime_B.M_Slime_B")
              (Variables|/Game/UI/Dialogues/D_Z0/D_Base.D_Base_C|SetTextureID _output_get "/Game/Characters/NPCs/Slime_Green.Slime_Green")
              (UserInterface|Viewport|AddtoViewport _output_get 0 :!label _label_2)
              (goto _label)
              (elif (== (Rendering|Material|GetMaterial (Variables|Character|GetMesh) 0) "/Game/Characters/NPCs/M_Slime_C.M_Slime_C")
                (Variables|/Game/UI/Dialogues/D_Z0/D_Base.D_Base_C|SetTextureID _output_get "/Game/Characters/NPCs/Slime_Red.Slime_Red")
                (goto _label_2)
                (elif (== (Rendering|Material|GetMaterial (Variables|Character|GetMesh) 0) "/Game/Characters/NPCs/M_Slime_D.M_Slime_D")
                  (Variables|/Game/UI/Dialogues/D_Z0/D_Base.D_Base_C|SetTextureID _output_get "/Game/Characters/NPCs/Slime_Blue.Slime_Blue")
                  (goto _label_2)
                  (elif (== (Rendering|Material|GetMaterial (Variables|Character|GetMesh) 0) "/Game/Characters/NPCs/M_Slime_E.M_Slime_E")
                    (Variables|/Game/UI/Dialogues/D_Z0/D_Base.D_Base_C|SetTextureID _output_get "/Game/Characters/NPCs/Slime_Rosa.Slime_Rosa")
                    (goto _label_2)
                    (elif (== (Rendering|Material|GetMaterial (Variables|Character|GetMesh) 0) "/Game/Characters/NPCs/M_Slime_F.M_Slime_F")
                      (Variables|/Game/UI/Dialogues/D_Z0/D_Base.D_Base_C|SetTextureID _output_get "/Game/Characters/NPCs/Slime_Yellow.Slime_Yellow")
                      (goto _label_2))))))))
        (else
          (bind _asmain_slime_character_2 (Utilities|Casting|CastToMainSlimeCharacter (Game|GetPlayerCharacter 0)))
          (Variables|/Script/Engine.CharacterMovementComponent|SetMaxWalkSpeed (Variables|/Script/Engine.Character|GetCharacterMovement _asmain_slime_character_2) 7e+02)
          (Widget|RemovefromParent (Variables|Default|GetUI_Base))
          (Rendering|SetVisibility (Variables|Default|GetWidget) false false)
          (Variables|/Game/Core/Blueprints/MainSlimeCharacter.MainSlimeCharacter_C|SetIsInDialogue _asmain_slime_character_2 false))))))

(fn ConstructionScript)