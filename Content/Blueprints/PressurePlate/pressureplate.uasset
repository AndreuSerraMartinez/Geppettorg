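; One-shot pressure plate that magnetically captures a slime piece to activate a linked door.
; The first piece entering the sphere is removed from the slime character, then pulled in by a delayed recursive velocity loop until close enough to snap.
; Chained timelines seat the piece, lower the plate and recolor its light, then trigger the door, destroy the piece and leave the stone spinning.
; Older switch and piece-search logic remains disconnected.
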(event OnComponentBeginOverlap(SphereRangeMagnet)
  (params (OverlappedComponent :type Primitive%20Component%20Object%20Reference) (OtherActor :type Actor%20Object%20Reference) (OtherComp :type Primitive%20Component%20Object%20Reference) (OtherBodyIndex :type Integer) (bFromSweep :type Boolean) (SweepResult :type Hit%20Result%20Structure%20%28by%20ref%29))
  (bind _aspieces (Utilities|Casting|CastToPieces OtherActor))
  (Utilities|FlowControl|DoOnce false
    (:Completed
      (Variables|Default|SetPieceToMagnet _aspieces)
      (bind _asmain_slime_character (Utilities|Casting|CastToMainSlimeCharacter (Game|GetPlayerCharacter 0)))
      (Default|DeleteChunk _asmain_slime_character (Variables|Default|GetPieceToMagnet))
      (Audio|PlaySoundatLocation "/Game/Sounds/SFX/SoundsBeta/Sound_Design/Others/Press/Press_Plate_2.Press_Plate_2" (Transformation|GetActorLocation) "0, 0, 0" 1.0 1.0 0.0 "/Game/Sounds/SFX/AttenuationSetting3DSound.AttenuationSetting3DSound" 0 0 0)
      (CallFunction|MagnetPiece))))

(event OnComponentEndOverlap(SphereRangeMagnet)
  (params (OverlappedComponent :type Primitive%20Component%20Object%20Reference) (OtherActor :type Actor%20Object%20Reference) (OtherComp :type Primitive%20Component%20Object%20Reference) (OtherBodyIndex :type Integer))
  (if (== OtherActor (Variables|Default|GetPieceToMagnet))
    (Variables|Default|SetPieceToMagnet 0)))

(event Custom|SearchForPieces)

(event Custom|MagnetPiece
  (if (Utilities|IsValid (Variables|Default|GetPieceToMagnet))
    (if (< (Math|Vector|Distance(Vector) (Transformation|GetWorldLocation (Variables|Default|GetSphereRangeMagnet)) (Transformation|GetActorLocation (Variables|Default|GetPieceToMagnet))) 1.2e+02)
      (Variables|Default|SetInitPieceLocation (Transformation|GetActorLocation (Variables|Default|GetPieceToMagnet)))
      (Audio|PlaySoundatLocation "/Game/Sounds/SFX/SoundsBeta/New_Zone.New_Zone" (Transformation|GetActorLocation) "0, 0, 0" 0.8 1.0 0.0 "/Game/Sounds/SFX/AttenuationSetting3DSound.AttenuationSetting3DSound" 0 0 0)
      (bind _newtrack_0 (Timeline|SnapPiece PlayFromStart)
        (:Update
          (Transformation|SetActorLocation (Variables|Default|GetPieceToMagnet) (Math|Vector|Lerp(Vector) (Variables|Default|GetInitPieceLocation) (Transformation|GetWorldLocation (Variables|Default|GetArrow)) _newtrack_0) false false)
          (Transformation|AddLocalRotation (Variables|Default|GetStone) (Math|Rotator|MakeRotator 0.0 0.0 (* (Utilities|Time|GetWorldDeltaSeconds) 6e+01)) false false))
        (:Finished
          (bind (_direction _switchpos _newtrack_0_2) (Timeline|LowerPlate PlayFromStart)
            (:Update
              (Transformation|SetRelativeLocation (Variables|Default|GetPlate) (Math|Vector|MakeVector 0.0 0.0 _switchpos) false false)
              (Rendering|Components|Light|SetLightColor (Variables|Default|GetPointLight) _newtrack_0_2 true)
              (Rendering|Material|SetVectorParameterValueonMaterials (Variables|Default|GetLightSurface) "Color" (Math|Conversions|ToVector(LinearColor) _newtrack_0_2))
              (Transformation|AddLocalRotation (Variables|Default|GetStone) (Math|Rotator|MakeRotator 0.0 0.0 (* (Utilities|Time|GetWorldDeltaSeconds) 6e+01)) false false))
            (:Finished
              (Default|PressureActivated (Variables|Default|GetDoorToActivate))
              (Variables|Default|SetActive true)
              (Audio|PlaySound2D "/Game/Sounds/SFX/Press_plate_Cue.Press_plate_Cue" 1.2 1.0 0.0 0 0)
              (Default|Die (Variables|Default|GetPieceToMagnet))
              (Variables|Default|SetPieceToMagnet 0)
              (Components|Activation|SetActive (Variables|Default|GetPreasurePlateActive) true false)))))
      (else
        ;[1 0.963 0] Forces
        (Physics|SetPhysicsLinearVelocity (Variables|/Game/Core/Blueprints/Pieces.Pieces_C|GetSphere1 (Variables|Default|GetPieceToMagnet)) (* (Math|Vector|GetUnitDirection(Vector) (Transformation|GetActorLocation (Variables|Default|GetPieceToMagnet)) (Transformation|GetWorldLocation (Variables|Default|GetSphereRangeMagnet))) 4e+02) false "None")
        (Utilities|FlowControl|Delay 0.2)
        (CallFunction|MagnetPiece)
        (Transformation|AddLocalRotation (Variables|Default|GetStone) (Math|Rotator|MakeRotator 0.0 0.0 (* (Utilities|Time|GetWorldDeltaSeconds) 6e+01)) false false)))
    (else
      (Variables|Default|SetPieceToMagnet 0))))

(event EventBeginPlay)

(event Collision|EventActorBeginOverlap
  (params (OtherActor :type Actor%20Object%20Reference)))

(event EventTick
  (params (DeltaSeconds :type Float%20%28single-precision%29))
  (if (Variables|Default|GetActive)
    (Transformation|AddLocalRotation (Variables|Default|GetStone) (Math|Rotator|MakeRotator 0.0 0.0 (* (Utilities|Time|GetWorldDeltaSeconds) 1e+01)) false false)))

(event Collision|EventActorEndOverlap
  (params (OtherActor :type Actor%20Object%20Reference)))

(fn ConstructionScript)