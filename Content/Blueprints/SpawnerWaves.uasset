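; Arena wave spawner that starts once when the slime player enters its sphere, activating its SpawnerWalls.
; Waves spawn after a delay at random navigable points, with each supported enemy given a spawner reference.
; CheckEnemyLeft triggers the next wave when none remain alive.
; Manual mode follows WavesPool, toggles the GameInstance attack-zone flag and drops walls when finished; automatic mode spawns endless, growing random waves from TypePool.
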(event OnComponentBeginOverlap(SphereRange)
  (params (OverlappedComponent :type Primitive%20Component%20Object%20Reference) (OtherActor :type Actor%20Object%20Reference) (OtherComp :type Primitive%20Component%20Object%20Reference) (OtherBodyIndex :type Integer) (bFromSweep :type Boolean) (SweepResult :type Hit%20Result%20Structure%20%28by%20ref%29))
  (Utilities|Casting|CastToMainSlimeCharacter OtherActor)
  (Utilities|FlowControl|DoOnce false
    (:Completed
      (CallFunction|SpawnEnemy)
      (CallFunction|CheckEnemyLeft)
      (for _array_element (Variables|Manual|GetWalls)
        (bind _asspawner_walls (Utilities|Casting|CastToSpawnerWalls _array_element))
        (Default|ActiveInactive _asspawner_walls true)))))

(event Custom|CheckEnemyLeft
  (if (== (Variables|Default|GetEnemyAlive) 0)
    (CallFunction|SpawnEnemy)))

(event Custom|SpawnEnemy
  (bind _wavespool (Variables|Manual|GetWavesPool))
  (bind _wavenumber (Variables|Manual|GetWaveNumber))
  (Utilities|FlowControl|Sequence
    (:then_0
      (Utilities|FlowControl|Delay 2.0)
      (if (Variables|Default|GetManualWaves)
        ;[1 0.007639 0] Manual
        (if (Utilities|Array|IsValidIndex _wavespool _wavenumber)
          (Variables|Default|SetEnemyAlive 0)
          (for _array_element (Utilities|Struct|BreakWaveEnemies (Utilities|Array|Get(acopy) _wavespool _wavenumber))
            (Math|Integer|IncrementInt (Variables|Default|GetEnemyAlive)
              (:%20%20
                (bind _randomlocation (Class|NavigationSystemV1|GetRandomLocationinNavigableRadius (.location (Transformation|GetActorTransform)) (Variables|/Script/Engine.SphereComponent|GetSphereRadius (Variables|Default|GetSphereRange)) 0 0))
                (bind _returnvalue (Game|SpawnActorfromClass _array_element (Math|Transform|MakeTransform _randomlocation (Math|Rotator|MakeRotator 0.0 0.0 (.yaw (Math|Random|RandomRotator false))) "1.000000,1.000000,1.000000") "AdjustIfPossibleButAlwaysSpawn" 0 0))
                (bind _ascorrupted_armadillo (Utilities|Casting|CastToCorruptedArmadillo _returnvalue)
                  (:then
                    (Variables|/Game/Characters/Enemies/Armadillo/CorruptedArmadillo.CorruptedArmadillo_C|SetSpawner _ascorrupted_armadillo self)
                    (Variables|/Game/Characters/Enemies/Armadillo/CorruptedArmadillo.CorruptedArmadillo_C|SetSpawned _ascorrupted_armadillo true))
                  (:CastFailed
                    (bind _asbp_cactus (Utilities|Casting|CastToBP_Cactus _returnvalue)
                      (:then
                        (Variables|/Game/Characters/Enemies/Cactus/BP_Cactus.BP_Cactus_C|SetSpawner _asbp_cactus self)
                        (Variables|/Game/Characters/Enemies/Cactus/BP_Cactus.BP_Cactus_C|SetSpawned _asbp_cactus true))
                      (:CastFailed
                        (bind _asgoblin (Utilities|Casting|CastToGoblin _returnvalue))
                        (Variables|/Game/Characters/Enemies/Goblin/Goblin.Goblin_C|SetSpawner _asgoblin self)
                        (Variables|/Game/Characters/Enemies/Goblin/Goblin.Goblin_C|SetSpawned _asgoblin true))))))))
          (Math|Integer|IncrementInt (Variables|Manual|GetWaveNumber))
          (else
            (for _array_element_2 (Variables|Manual|GetWalls)
              (bind _asspawner_walls (Utilities|Casting|CastToSpawnerWalls _array_element_2))
              (Default|ActiveInactive _asspawner_walls false))
            (Variables|/Game/Blueprints/SlimeGameInstance.SlimeGameInstance_C|SetAtackZone (Variables|Default|GetAs%20Slime%20Game%20Instance) false)))
        (else
          ;[0 0.1516 1] Automatic
          (for _index (range 0 (- (Variables|Automatic|GetEnemiesXWave) 1))
            (bind _randomlocation_2 (Class|NavigationSystemV1|GetRandomLocationinNavigableRadius (.location (Transformation|GetActorTransform)) (Variables|/Script/Engine.SphereComponent|GetSphereRadius (Variables|Default|GetSphereRange)) 0 0))
            (bind _returnvalue_2 (Game|SpawnActorfromClass (.OutItem (Utilities|Array|Random (Variables|Default|GetTypePool))) (Math|Transform|MakeTransform _randomlocation_2 (Math|Rotator|MakeRotator 0.0 0.0 (.yaw (Math|Random|RandomRotator false))) "1.000000,1.000000,1.000000") "Undefined" 0 0))
            (bind _ascorrupted_armadillo_2 (Utilities|Casting|CastToCorruptedArmadillo _returnvalue_2)
              (:then
                (Variables|/Game/Characters/Enemies/Armadillo/CorruptedArmadillo.CorruptedArmadillo_C|SetSpawner _ascorrupted_armadillo_2 self)
                (Variables|/Game/Characters/Enemies/Armadillo/CorruptedArmadillo.CorruptedArmadillo_C|SetSpawned _ascorrupted_armadillo_2 true))
              (:CastFailed
                (bind _asbp_cactus_2 (Utilities|Casting|CastToBP_Cactus _returnvalue_2)
                  (:then
                    (Variables|/Game/Characters/Enemies/Cactus/BP_Cactus.BP_Cactus_C|SetSpawner _asbp_cactus_2 self)
                    (Variables|/Game/Characters/Enemies/Cactus/BP_Cactus.BP_Cactus_C|SetSpawned _asbp_cactus_2 true))
                  (:CastFailed
                    (bind _asgoblin_2 (Utilities|Casting|CastToGoblin _returnvalue_2))
                    (Variables|/Game/Characters/Enemies/Goblin/Goblin.Goblin_C|SetSpawner _asgoblin_2 self)
                    (Variables|/Game/Characters/Enemies/Goblin/Goblin.Goblin_C|SetSpawned _asgoblin_2 true))))))
          (Variables|Default|SetEnemyAlive (Variables|Automatic|GetEnemiesXWave))
          (Variables|Automatic|SetEnemiesXWave (+ (Variables|Automatic|GetEnemiesXWave) (Variables|Automatic|GetIncrementOfEnemiesXWave))))))
    (:then_1
      (if (Variables|Default|GetManualWaves)
        (Variables|/Game/Blueprints/SlimeGameInstance.SlimeGameInstance_C|SetAtackZone (Variables|Default|GetAs%20Slime%20Game%20Instance) true)))))

(event EventBeginPlay
  (bind _asslime_game_instance (Utilities|Casting|CastToSlimeGameInstance (Game|GetGameInstance)))
  (Variables|Default|SetAs%20Slime%20Game%20Instance _asslime_game_instance))

(fn ConstructionScript)