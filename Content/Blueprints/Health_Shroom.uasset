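; Health mushroom pickup that restores life to the main slime character on overlap and respawns after a delay.
; An Active flag blocks repeat pickups while it plays the eat sound and a timeline animates the mushroom's scale before hiding the actor.
; After the respawn timer, it reappears, a second timeline played in reverse animates the scale back, and the pickup becomes active again.
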(event Collision|EventActorBeginOverlap
  (params (OtherActor :type Actor%20Object%20Reference))
  (bind _asmain_slime_character (Utilities|Casting|CastToMainSlimeCharacter OtherActor))
  (if (Variables|Default|GetActive)
    (Default|AddLife _asmain_slime_character 0.4)
    (Audio|PlaySoundatLocation "/Game/Sounds/SFX/SoundsBeta/Sound_Design/Characters/Slime/Eat_plant/Eat_plant.Eat_plant" (Transformation|GetActorLocation) "0, 0, 0" 1.0 1.0 0.0 0 0 0 0)
    (Variables|Default|SetActive false)
    (bind _newtrack_0 (Timeline|Timeline_0 PlayFromStart)
      (:Update
        (Transformation|SetRelativeScale3D (Variables|Default|GetShroom) (Math|Conversions|ToVector(Float) _newtrack_0)))
      (:Finished
        (Rendering|SetActorHiddenInGame true)
        (Utilities|FlowControl|Delay (Variables|Default|GetTimerRespawn))
        (Rendering|SetActorHiddenInGame false)
        (bind _newtrack_0_2 (Timeline|Timeline ReverseFromEnd)
          (:Update
            (Transformation|SetRelativeScale3D (Variables|Default|GetShroom) (Math|Conversions|ToVector(Float) _newtrack_0_2)))
          (:Finished
            (Variables|Default|SetActive true)))))))

(fn ConstructionScript)