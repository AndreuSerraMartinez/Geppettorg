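; A door actor that opens once enough pressure activators are triggered, counting activations against a required number.
; Activation and deactivation events adjust the count and play or reverse a timeline that moves the door vertically.
; Each timeline update also fires a camera shake at the slime character's camera and spawns a stone door sound.
; Camera-switching logic for a temporary view change is present but unconnected.
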(event Custom|PressureActivated
  (Math|Integer|IncrementInt (Variables|Default|GetPresureActivated)
    (:%20%20
      (if (>= (Variables|Default|GetPresureActivated) (Variables|Default|GetPressureNeeded))
        (bind _doorpos (Timeline|DoorActivate Play)
          (:Update
            (bind _asmain_slime_character (Utilities|Casting|CastToMainSlimeCharacter (Game|GetPlayerCharacter 0)))
            (Camera|PlayWorldCameraShake "/Game/Blueprints/Event/Door_Shake.Door_Shake_C" (Transformation|GetWorldLocation (Variables|/Game/Core/Blueprints/MainSlimeCharacter.MainSlimeCharacter_C|GetCamera _asmain_slime_character)) 0.0 5e+02)
            (Transformation|SetRelativeLocation (Variables|Default|GetDoor) (Math|Vector|MakeVector 0.0 0.0 _doorpos) false false)
            (Audio|SpawnSoundatLocation "/Game/Sounds/SFX/Stone_Door_cut.Stone_Door_cut" (Transformation|GetWorldLocation (Variables|Default|GetDoor)) "0, 0, 0" 0.5 1.0 0.0 0 0)))))))

(event Custom|Switch%20Deactivated
  (Math|Integer|DecrementInt (Variables|Default|GetPresureActivated)
    (:%20%20
      (if (>= (Variables|Default|GetPresureActivated) (Variables|Default|GetPressureNeeded))
        (bind _doorpos (Timeline|DoorActivate Play)
          (:Update
            (bind _asmain_slime_character (Utilities|Casting|CastToMainSlimeCharacter (Game|GetPlayerCharacter 0)))
            (Camera|PlayWorldCameraShake "/Game/Blueprints/Event/Door_Shake.Door_Shake_C" (Transformation|GetWorldLocation (Variables|/Game/Core/Blueprints/MainSlimeCharacter.MainSlimeCharacter_C|GetCamera _asmain_slime_character)) 0.0 5e+02)
            (Transformation|SetRelativeLocation (Variables|Default|GetDoor) (Math|Vector|MakeVector 0.0 0.0 _doorpos) false false)
            (Audio|SpawnSoundatLocation "/Game/Sounds/SFX/Stone_Door_cut.Stone_Door_cut" (Transformation|GetWorldLocation (Variables|Default|GetDoor)) "0, 0, 0" 0.5 1.0 0.0 0 0)))
        (else
          (Timeline|DoorActivate Reverse))))))

(fn ConstructionScript)