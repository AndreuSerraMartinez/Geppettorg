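; BossFadeOut is an end-of-sequence trigger that stages a boss appearance and then returns the game to the main menu.
; When MainSlimeCharacter overlaps it, it sets a negative max walk speed, disables dashing and spawns a Boss at its own location.
; Two chained delays then lead to opening the MainMenu level.
; The widget creation, presumably the fade, and the self-destroy nodes are disconnected, so neither runs.
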(event EventBeginPlay)

(event Collision|EventActorBeginOverlap
  (params (OtherActor :type Actor%20Object%20Reference))
  (bind _asmain_slime_character (Utilities|Casting|CastToMainSlimeCharacter OtherActor))
  (bind _output_get (Variables|Default|SetAs%20Main%20Slime%20Character _asmain_slime_character))
  (Variables|/Script/Engine.CharacterMovementComponent|SetMaxWalkSpeed (Variables|/Script/Engine.Character|GetCharacterMovement _output_get) -1e+03)
  (Variables|/Game/Core/Blueprints/MainSlimeCharacter.MainSlimeCharacter_C|SetCanDash _output_get false)
  (Game|SpawnActorfromClass "/Game/Characters/Enemies/Boss/Boss.Boss_C" (Math|Transform|MakeTransform (Transformation|GetActorLocation) "0, 0, 0" "1.000000,1.000000,1.000000") "Undefined" 0 0)
  (Utilities|FlowControl|Delay 5.0)
  (Utilities|FlowControl|Delay 3.0)
  (Game|OpenLevel(byObjectReference) "/Game/LEVELS/MainMenu.MainMenu"))

(event EventTick
  (params (DeltaSeconds :type Float%20%28single-precision%29)))

(fn ConstructionScript)