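; NewZone is a one-shot trigger volume that announces a new zone to the player with an on-screen title and a sound.
; Its box overlap passes a DoOnce, then casts to MainSlimeCharacter, so the first overlapping actor of any kind consumes the trigger.
; For the slime, it shows a NewZone_Widget carrying its TITLEText, plays the New_Zone sound after a short delay, then removes the widget seconds later.
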(event OnComponentBeginOverlap(Box)
  (params (OverlappedComponent :type Primitive%20Component%20Object%20Reference) (OtherActor :type Actor%20Object%20Reference) (OtherComp :type Primitive%20Component%20Object%20Reference) (OtherBodyIndex :type Integer) (bFromSweep :type Boolean) (SweepResult :type Hit%20Result%20Structure%20%28by%20ref%29))
  (Utilities|FlowControl|DoOnce false
    (:Completed
      (Utilities|Casting|CastToMainSlimeCharacter OtherActor)
      (bind _returnvalue (UserInterface|CreateWidget "/Game/Blueprints/Widgets/NewZone_Widget.NewZone_Widget_C" (Game|GetPlayerController 0) (Variables|Default|GetTITLE%20text)))
      (bind _output_get (Variables|Default|SetUI_NewZone _returnvalue))
      (UserInterface|Viewport|AddtoViewport _output_get 0)
      (Utilities|FlowControl|Delay 0.5)
      (Audio|PlaySound2D "/Game/Sounds/SFX/SoundsBeta/New_Zone.New_Zone" 1.0 1.0 0.0 0 0)
      (Utilities|FlowControl|Delay 5.0)
      (Widget|RemovefromParent _returnvalue))))

(event EventBeginPlay)

(event Collision|EventActorBeginOverlap
  (params (OtherActor :type Actor%20Object%20Reference)))

(event EventTick
  (params (DeltaSeconds :type Float%20%28single-precision%29)))

(fn ConstructionScript)