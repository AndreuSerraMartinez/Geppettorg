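; Demon Door is a barrier that stays until every actor in its EnemiesToDefeat list is gone.
; When In is set, BeginPlay enables collision on the Cube and fades in a dynamic DarkDoor material through a timeline.
; Tick checks the list and calls Deactivate every frame once none are valid.
; Deactivate disables collision, recreates the material, fades its opacity by timeline and destroys the actor after a delay started from the timeline's update.
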(event Custom|Deactivate
  (Collision|SetCollisionEnabled (Variables|Default|GetCube) "NoCollision")
  (bind _returnvalue (Rendering|Material|CreateDynamicMaterialInstance (Variables|Default|GetCube) 0 "/Game/MaterialsLibrary/DarkDoor.DarkDoor" "None" :!class /Script/Engine.PrimitiveComponent))
  (bind _output_get (Variables|Default|SetMID _returnvalue))
  (Rendering|Material|SetMaterial (Variables|Default|GetCube) 0 _output_get)
  (bind _opacitytrack2 (Timeline|FadeOutTimeline Play)
    (:Update
      (Rendering|Material|SetScalarParameterValue (Variables|Default|GetMID) "Opacity" _opacitytrack2 :!class /Script/Engine.MaterialInstanceDynamic)
      (Utilities|FlowControl|Delay 1.5)
      (Actor|DestroyActor))))

(event EventBeginPlay
  (if (Variables|Default|GetIn)
    (Collision|SetCollisionEnabled (Variables|Default|GetCube) "QueryAndPhysics")
    (bind _returnvalue (Rendering|Material|CreateDynamicMaterialInstance (Variables|Default|GetCube) 0 "/Game/MaterialsLibrary/DarkDoor.DarkDoor" "None" :!class /Script/Engine.PrimitiveComponent))
    (bind _output_get (Variables|Default|SetMID _returnvalue))
    (Rendering|Material|SetMaterial (Variables|Default|GetCube) 0 _output_get)
    (bind _opacitytrack (Timeline|FadeInTimeline Play)
      (:Update
        (Rendering|Material|SetScalarParameterValue (Variables|Default|GetMID) "Opacity" _opacitytrack :!class /Script/Engine.MaterialInstanceDynamic)))))

(event EventTick
  (params (DeltaSeconds :type Float%20%28single-precision%29))
  (Variables|Default|SetEnemiesAlive? false)
  (for _array_element (Variables|Default|GetEnemiesToDefeat)
    (Utilities|IsValid _array_element
      (:Is%20Valid
        (Variables|Default|SetEnemiesAlive? true))))
  (if (not (Variables|Default|GetEnemiesAlive?))
    (CallFunction|Deactivate)))

(fn ConstructionScript)