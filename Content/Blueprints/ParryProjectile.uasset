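; ParryProjectile is a projectile actor, by its name tied to parrying, that damages enemies it touches.
; When Sphere1 begins an overlap, it tries casts to Enemy3_mele and Enemy1 and calls DMG on a match.
; SetPLayer stores a player character reference, used only by an unconnected impulse toward that player.
; DestroyProjectile removes the actor but is not called here, so overlaps do not destroy it.
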(event OnComponentBeginOverlap(Sphere1)
  (params (OverlappedComponent :type Primitive%20Component%20Object%20Reference) (OtherActor :type Actor%20Object%20Reference) (OtherComp :type Primitive%20Component%20Object%20Reference) (OtherBodyIndex :type Integer) (bFromSweep :type Boolean) (SweepResult :type Hit%20Result%20Structure%20%28by%20ref%29))
  (Utilities|FlowControl|Sequence
    (:then_0
      (bind _asenemy_3_mele (Utilities|Casting|CastToEnemy3_mele OtherActor))
      (Default|DMG _asenemy_3_mele))
    (:then_1
      (bind _asenemy_1 (Utilities|Casting|CastToEnemy1 OtherActor))
      (Default|DMG _asenemy_1))))

(event Custom|SetPLayer
  (params (NewParam :type BP%20Third%20Person%20Character%20Object%20Reference))
  (bind _output_get (Variables|Default|SetAs%20BP%20Third%20Person%20Character NewParam)))

(fn ConstructionScript)

(fn DestroyProjectile
  (Actor|DestroyActor))