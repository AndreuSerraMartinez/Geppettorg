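; Melee enemy Blueprint that chases the player and attacks at close range, with a widget health bar tracking its HP.
; Seeing a pawn through PawnSensing starts an AI move to the player; on arrival, a CanAttack-gated sequence briefly shows the AttackSpace area and swaps its material.
; Midway through that timed attack, an overlapping player character gets SplitLife called.
; The DMG event decrements HP, updates the bar and destroys the enemy at zero.
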(event OnSeePawn(PawnSensing)
  (params (Pawn :type Pawn%20Object%20Reference))
  (Variables|Default|SetInSensingPlayer true)
  (CallFunction|FollowPlayer))

(event Custom|FollowPlayer
  (if true
    (AI|AIMoveTo self "0, 0, 0" (Game|GetPlayerCharacter 0) 7e+01 false
      (:OnSuccess
        (if (Variables|Default|GetCanAttack)
          (Variables|Default|SetCanAttack false)
          (Animation|PlayAnimMontage 0 1.0 "None")
          ;[1 1 1] Anim attack
          (Development|SetHiddeninGame (Variables|Default|GetAttackSpace) false false)
          (Utilities|FlowControl|Delay 0.4)
          (Rendering|Material|SetMaterial (Variables|Default|GetAttackSpace) 0 "/Game/Custom_Mats/DemonEnclose.DemonEnclose")
          (bind _asbp_third_person_character (Utilities|Casting|CastToBP_ThirdPersonCharacter (Utilities|Array|Get(acopy) (Collision|GetOverlappingActors (Variables|Default|GetAttackSpace) "/Game/ThirdPerson/Blueprints/BP_ThirdPersonCharacter.BP_ThirdPersonCharacter_C" :!class /Script/Engine.PrimitiveComponent)))
            (:then
              (Default|SplitLife _asbp_third_person_character))
            (:CastFailed
              _))
          (Utilities|FlowControl|Delay 0.2)
          (Rendering|Material|SetMaterial (Variables|Default|GetAttackSpace) 0 "/Game/Characters/Slime/Fwd.Fwd")
          (Development|SetHiddeninGame (Variables|Default|GetAttackSpace) true false)
          (Variables|Default|SetCanAttack true))))))

(event Custom|DMG
  (Math|Integer|DecrementInt (Variables|Default|GetHP)
    (:%20%20
      (Variables|/Game/Blueprints/HealthBar.HealthBar_C|SetHealth (Variables|Default|GetHealthBar) (Math|Conversions|ToFloat(Integer) (Variables|Default|GetHP)))
      (if (<= (Variables|Default|GetHP) 0)
        (Actor|DestroyActor)))))

(event EventBeginPlay
  (Development|SetHiddeninGame (Variables|Default|GetAttackSpace) true false)
  (bind _ashealth_bar (Utilities|Casting|CastToHealthBar (UserInterface|GetUserWidgetObject (Variables|Default|GetWidget))))
  (bind _output_get (Variables|Default|SetHealthBar _ashealth_bar))
  (bind _output_get_2 (Variables|/Game/Blueprints/HealthBar.HealthBar_C|SetMaxHealth _output_get (Math|Conversions|ToFloat(Integer) (Variables|Default|GetHP))))
  (Variables|/Game/Blueprints/HealthBar.HealthBar_C|SetHealth _output_get _output_get_2))

(event Collision|EventActorBeginOverlap
  (params (OtherActor :type Actor%20Object%20Reference)))

(event EventTick
  (params (DeltaSeconds :type Float%20%28single-precision%29)))

(fn ConstructionScript)