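; SpawnerWalls is a toggleable barrier actor made of a Niagara effect and a box collider.
; The ActiveInactive event stores the Active flag, then shows or hides the effect and switches the box between query-and-physics and no collision to match.
; BeginPlay calls it with false, so the wall starts invisible and passable.
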(event Custom|ActiveInactive
  (params (Active :type Boolean))
  (bind _box (Variables|Default|GetBox))
  (bind _niagara (Variables|Default|GetNiagara))
  (Variables|Default|SetActive Active)
  (if (Variables|Default|GetActive)
    (Rendering|SetVisibility _niagara true false)
    (Collision|SetCollisionEnabled _box "QueryAndPhysics")
    (else
      (Rendering|SetVisibility _niagara false false)
      (Collision|SetCollisionEnabled _box "NoCollision"))))

(event EventBeginPlay
  (CallFunction|ActiveInactive false))

(event Collision|EventActorBeginOverlap
  (params (OtherActor :type Actor%20Object%20Reference)))

(event EventTick
  (params (DeltaSeconds :type Float%20%28single-precision%29)))

(fn ConstructionScript)