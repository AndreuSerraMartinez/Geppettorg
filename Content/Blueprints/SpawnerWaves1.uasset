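; SpawnerWaves1 is an enemy spawner actor that spawns a single CorruptedArmadillo at its own transform on BeginPlay.
; Despite the name, the active graph has no wave, timer or repeat logic.
; Disconnected nodes hold a second spawn and a cast chain for CorruptedArmadillo, BP_Cactus and Goblin that would set Spawner and Spawned.
; Those nodes never run, so the spawned enemy receives neither value from this Blueprint.
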(event EventBeginPlay
  (Game|SpawnActorfromClass "/Game/Characters/Enemies/Armadillo/CorruptedArmadillo.CorruptedArmadillo_C" (Transformation|GetActorTransform) "Undefined" 0 0))

(fn ConstructionScript)