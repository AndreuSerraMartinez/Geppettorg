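; Enemy1 is a turret-like enemy that turns to face the player character and repeatedly fires projectiles at them.
; On BeginPlay it caches the BP_ThirdPersonCharacter player reference.
; Each Tick it rotates the whole actor with a look-at from its SpawnProjectile point, then, if CanShoot allows, spawns a Projectile1 there and passes it the player.
; A Delay on Cooldown re-arms CanShoot, with no range or line-of-sight check.
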(event EventBeginPlay
  (bind _asbp_third_person_character (Utilities|Casting|CastToBP_ThirdPersonCharacter (Game|GetPlayerCharacter 0)))
  (Variables|Default|SetAs%20BP%20Third%20Person%20Character _asbp_third_person_character))

(event Collision|EventActorBeginOverlap
  (params (OtherActor :type Actor%20Object%20Reference)))

(event EventTick
  (params (DeltaSeconds :type Float%20%28single-precision%29))
  (Transformation|SetActorRotation (Math|Rotator|FindLookatRotation (Transformation|GetWorldLocation (Variables|Default|GetSpawn_projectile)) (.location (Transformation|GetActorTransform (Variables|Default|GetAs%20BP%20Third%20Person%20Character)))))
  (if (Variables|Default|GetCanShoot)
    (Variables|Default|SetCanShoot false)
    (bind _returnvalue (Game|SpawnActorfromClass "/Game/Blueprints/Projectile1.Projectile1_C" (Transformation|GetWorldTransform (Variables|Default|GetSpawn_projectile)) "Undefined" 0 0))
    (Default|SetPLayer _returnvalue (Variables|Default|GetAs%20BP%20Third%20Person%20Character))
    (Utilities|FlowControl|Delay (Variables|Default|GetCooldown))
    (Variables|Default|SetCanShoot true)))

(fn ConstructionScript)