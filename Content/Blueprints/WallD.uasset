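; WallD is a destructible wall that the slime player character breaks with its fist collision, provided the character's Life is above 0.7.
; Fist overlaps on Box1 during a slash decrement the wall's Life, playing Niagara debris VFX and swapping to another mesh until it runs out.
; At zero Life, or on a non-slash fist hit while CanDash is false, a DoOnce destroys the wall components with VFX and rock-breaking sound.
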(event OnComponentBeginOverlap(Box1)
  (params (OverlappedComponent :type Primitive%20Component%20Object%20Reference) (OtherActor :type Actor%20Object%20Reference) (OtherComp :type Primitive%20Component%20Object%20Reference) (OtherBodyIndex :type Integer) (bFromSweep :type Boolean) (SweepResult :type Hit%20Result%20Structure%20%28by%20ref%29))
  (bind _life (Variables|Default|GetLife))
  (bind _asmain_slime_character (Utilities|Casting|CastToMainSlimeCharacter OtherActor))
  (if (> (Variables|/Game/Core/Blueprints/MainSlimeCharacter.MainSlimeCharacter_C|GetLife _asmain_slime_character) 0.7)
    (if (== (Variables|/Game/Core/Blueprints/MainSlimeCharacter.MainSlimeCharacter_C|GetFistSphereCollision _asmain_slime_character) OtherComp)
      (if (Variables|/Game/Core/Blueprints/MainSlimeCharacter.MainSlimeCharacter_C|GetSlashActive _asmain_slime_character)
        (Math|Integer|DecrementInt _life
          (:%20%20
            (if (> _life 0)
              (Components|Activation|Activate (Variables|Default|GetN_DestructibleWallVFX) true)
              (Components|StaticMesh|SetStaticMesh (Variables|Default|GetStaticMesh) "/Game/ArtPacks/LowPolyDungeons/Meshes/Dungeons/Mesh_Dungeons_Wall_21.Mesh_Dungeons_Wall_21")
              (else
                (Utilities|FlowControl|DoOnce false :!label _label
                  (:Completed
                    (Utilities|FlowControl|Sequence
                      (:then_1
                        (Components|DestroyComponent (Variables|Default|GetStaticMesh))
                        (Components|Activation|Activate (Variables|Default|GetN_DestructibleWallVFX) true)
                        (Audio|PlaySoundatLocation "/Game/Sounds/SFX/Rock_Breaking.Rock_Breaking" (Transformation|GetActorLocation) "0, 0, 0" 1.0 1.0 0.0 0 0 0 0)
                        (Components|DestroyComponent (Variables|Default|GetWall2))))))))))
        (elif (not (Variables|/Game/Core/Blueprints/MainSlimeCharacter.MainSlimeCharacter_C|GetCanDash _asmain_slime_character))
          (goto _label))))))

(event EventBeginPlay)

(event Collision|EventActorBeginOverlap
  (params (OtherActor :type Actor%20Object%20Reference)))

(event EventTick
  (params (DeltaSeconds :type Float%20%28single-precision%29)))

(fn ConstructionScript)