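; Melee enemy that faces its target and advances in timed steps, destroying itself when HP equals zero.
; Tick gates movement on seek range and cooldown, then retargets the closest Pieces actor, or the player if none exist.
; Each step lerps to the Arrow's position via the Move timeline, without sweep; the closest-distance value is never reset between searches.
; The box overlap only casts to Pieces and applies no effect.
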(event OnComponentBeginOverlap(BoxCollision)
  (params (OverlappedComponent :type Primitive%20Component%20Object%20Reference) (OtherActor :type Actor%20Object%20Reference) (OtherComp :type Primitive%20Component%20Object%20Reference) (OtherBodyIndex :type Integer) (bFromSweep :type Boolean) (SweepResult :type Hit%20Result%20Structure%20%28by%20ref%29))
  (Utilities|Casting|CastToPieces OtherActor))

(event EventBeginPlay
  (bind _asbp_third_person_character (Utilities|Casting|CastToBP_ThirdPersonCharacter (Game|GetPlayerCharacter 0)))
  (bind _output_get (Variables|Default|SetAs%20BP%20Third%20Person%20Character _asbp_third_person_character))
  (Variables|Default|SetTarget _output_get))

(event Collision|EventActorBeginOverlap
  (params (OtherActor :type Actor%20Object%20Reference)))

(event EventTick
  (params (DeltaSeconds :type Float%20%28single-precision%29))
  (CallFunction|Die@0HP)
  (Transformation|SetActorRotation (Math|Rotator|FindLookatRotation (Transformation|GetWorldLocation (Variables|Default|GetCone2)) (.location (Transformation|GetActorTransform (Variables|Default|GetTarget)))))
  ;[0 0.1146 0.00273] Move
  (if (>= (Variables|Default|GetSeekRange) (Math|Vector|VectorLength (- (Transformation|GetActorLocation (Variables|Default|GetTarget)) (Transformation|GetActorLocation))))
    (if (Variables|Default|GetCanMove)
      (Variables|Default|SetCanMove false)
      (bind _outactors (Actor|GetAllActorsOfClass "/Game/Characters/Slime/Pieces.Pieces_C"))
      (bind _output_get (Variables|Default|SetPieces%20Out%20Actors _outactors))
      (if (Utilities|Array|IsValidIndex _outactors)
        (for (_array_element _array_index) _output_get
          (if (< (Math|Vector|VectorLength (- (Transformation|GetActorLocation _array_element) (Transformation|GetActorLocation))) (Variables|Default|GetCloserDistancePiece))
            (Variables|Default|SetCloserDistancePiece (Math|Vector|VectorLength (- (Transformation|GetActorLocation _array_element) (Transformation|GetActorLocation))))
            (Variables|Default|SetCloserPiece _array_index)))
        (Variables|Default|SetTarget (Utilities|Array|Get(acopy) (Variables|Default|GetPieces%20Out%20Actors) (Variables|Default|GetCloserPiece)))
        (else
          (Variables|Default|SetTarget (Variables|Default|GetAs%20BP%20Third%20Person%20Character))))
      (Variables|Default|SetInitPos (Transformation|GetActorLocation))
      (Variables|Default|SetFinalPos (Transformation|GetWorldLocation (Variables|Default|GetArrow)))
      (bind _move (Timeline|Move PlayFromStart)
        (:Update
          (Transformation|SetActorLocation (Math|Vector|Lerp(Vector) (Variables|Default|GetInitPos) (Variables|Default|GetFinalPos) _move) false false))
        (:Finished
          (Utilities|FlowControl|Delay (Variables|Default|GetCooldown))
          (Variables|Default|SetCanMove true))))))

(fn ConstructionScript)

(fn Die@0HP
  (if (== (Variables|Default|GetHP) 0)
    (Actor|DestroyActor)))