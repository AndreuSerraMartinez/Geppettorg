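; Music actor for Zone 0 that starts the zone's Wwise music when play begins.
; On BeginPlay it casts the game instance to SlimeGameInstance and continues only if its SettingMusic flag is false.
; It then sets the level switch to level 0 and the gameplay state to idle, and posts the Play_z0 event on itself.
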(event EventBeginPlay
  (bind _asslime_game_instance (Utilities|Casting|CastToSlimeGameInstance (Game|GetGameInstance)))
  (if (not (Variables|/Game/Blueprints/SlimeGameInstance.SlimeGameInstance_C|GetSettingMusic _asslime_game_instance))
    (Class|AkGameplayStatics|SetSwitch "/Game/WwiseAudio/lvl_switch-lvl_0.lvl_switch-lvl_0" self (Variables|Default|GetSwitch%20group) (Variables|Default|GetSwitch%20State))
    (Class|AkGameplayStatics|SetState "/Game/WwiseAudio/gameplay_state-idle.gameplay_state-idle" (Variables|Default|GetState%20Group) (Variables|Default|GetState))
    (Class|AkGameplayStatics|PostEvent "/Game/WwiseAudio/Play_z0.Play_z0" self)))

(fn ConstructionScript)